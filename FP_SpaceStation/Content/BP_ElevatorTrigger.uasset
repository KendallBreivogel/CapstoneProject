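; BP_ElevatorTrigger is a rotating elevator trigger that turns a VR motion controller pawn along with it.
; Overlapping its box caches the first pawn, attaches it to the actor with world transforms kept, and plays a timeline.
; The timeline drives actor yaw by a curve-scaled Rotation from a quarter-turn base.
; On finish, it detaches the pawn and advances a position index that wraps through four 90-degree steps.
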(event `self.Box.OnComponentBeginOverlap`
  (params (OverlappedComponent :type "PrimitiveComponent Object Reference") (OtherActor :type "Actor Object Reference") (OtherComp :type "PrimitiveComponent Object Reference") (OtherBodyIndex :type Integer) (bFromSweep :type Boolean) (SweepResult :type "HitResult Structure (by ref)"))
  (bind _asmotion_controller_pawn (cast `/Game/VirtualRealityBP/Blueprints/MotionControllerPawn` OtherActor))
  (if (not (`KismetSystemLibrary.IsValid` (`self.Player`)))
    (set `self.Player` _asmotion_controller_pawn))
  (`self.RotateElevator`))

(event `RotateElevator`
  (bind _currentpos (`self.CurrentPos`))
  (`self.K2_AttachToActor` (`self.Player`) self "None" "KeepWorld" "KeepWorld" "KeepWorld" true)
  (bind (_direction _rotationovertime) (`Timeline|Rotate` :!via `PlayFromStart`)
    (:`Update`
      (`self.K2_SetActorRotation` (`KismetMathLibrary.MakeRotator` 0.0 0.0 (+ (* _rotationovertime (`self.Rotation`)) (* (`KismetMathLibrary.Conv_IntToDouble` (`self.CurrentPos`)) 90.0)))))
    (:`Finished`
      (`self.K2_DetachFromActor` (`self.Player`) "KeepWorld" "KeepWorld" "KeepWorld")
      (if (== _currentpos 3)
        (set `self.CurrentPos` 0)
        (else
          (`/Engine/EditorBlueprintResources/StandardMacros.IncrementInt` _currentpos))))))

(fn `UserConstructionScript`)