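; BP_Cookware is a cookware prop that can be picked up and dropped along with a grabbable object resting inside it.
; The InsideColl overlap events track one BP_Grabbable, which attaches to the cookware on pickup and is detached and dropped with it.
; Pickup turns off physics and swaps the collision channel while held, and Drop restores the channel and sets physics from its flags.
; The construction script applies mesh, grab box and optional random scale and yaw.
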(event `/Game/Blueprints/CharacterBPs/VirtualRealityBP/Blueprints/PickupActorInterface.Pickup`
  (params (AttachTo :type "SceneComponent Object Reference"))
  (bind _cube (`self.Cube`))
  (bind _insideobj (`self.InsideObj`))
  (if (`self.Pickupable`)
    (set `self.hasBeenPickedUp` true)
    (`PrimitiveComponent.SetSimulatePhysics` (`self.Cube`) false)
    (bind _output_get (set `self.AttachedComponent` AttachTo))
    (set `self.CollObjType` (`PrimitiveComponent.GetCollisionObjectType` _cube))
    (`PrimitiveComponent.SetCollisionObjectType` _cube "ECC_GameTraceChannel3")
    (`self.K2_AttachToComponent` _output_get "None" "KeepWorld" "KeepWorld" "KeepWorld")
    (if (`KismetSystemLibrary.IsValid` _insideobj)
      (`self.K2_AttachToActor` _insideobj self "None" "KeepWorld" "KeepWorld" "KeepWorld" true))))

(event `/Game/Blueprints/CharacterBPs/VirtualRealityBP/Blueprints/PickupActorInterface.Drop`
  (bind _insideobj (`self.InsideObj`))
  (`PrimitiveComponent.SetSimulatePhysics` (`self.Cube`) (or (`self.SimulatePhysics`) (`self.SimulatePhysicsOnDrop`)))
  (`self.K2_DetachFromActor` "KeepWorld" "KeepWorld" "KeepWorld")
  (`PrimitiveComponent.SetCollisionObjectType` (`self.Cube`) (`self.CollObjType`))
  (if (`KismetSystemLibrary.IsValid` _insideobj)
    (`self.K2_DetachFromActor` _insideobj "KeepWorld" "KeepWorld" "KeepWorld")
    (`/Game/Blueprints/CharacterBPs/VirtualRealityBP/Blueprints/PickupActorInterface.Drop` _insideobj)))

(event `self.InsideColl.OnComponentBeginOverlap`
  (params (OverlappedComponent :type "PrimitiveComponent Object Reference") (OtherActor :type "Actor Object Reference") (OtherComp :type "PrimitiveComponent Object Reference") (OtherBodyIndex :type Integer) (bFromSweep :type Boolean) (SweepResult :type "HitResult Structure (by ref)"))
  (bind _asbp_grabbable (cast `/Game/Blueprints/StationComponents/Templates/BP_Grabbable` OtherActor))
  (set `self.InsideObj` _asbp_grabbable))

(event `self.InsideColl.OnComponentEndOverlap`
  (params (OverlappedComponent :type "PrimitiveComponent Object Reference") (OtherActor :type "Actor Object Reference") (OtherComp :type "PrimitiveComponent Object Reference") (OtherBodyIndex :type Integer))
  (bind _asbp_grabbable (cast `/Game/Blueprints/StationComponents/Templates/BP_Grabbable` OtherActor))
  (if (== _asbp_grabbable (`self.InsideObj`))
    (set `self.InsideObj` null)))

(fn `UserConstructionScript`
  (bind _returnvalue (`KismetMathLibrary.RandomFloatInRange` 0.6 1.2))
  (bind _cube (`self.Cube`))
  (bind _cube_2 (`self.Cube`))
  (bind _box (`self.Box`))
  (`|ExecutionSequence`
    (:`then_0`
      (`PrimitiveComponent.SetSimulatePhysics` (`self.Cube`) (`self.SimulatePhysics`))
      (`StaticMeshComponent.SetStaticMesh` (`self.Cube`) (`self.Mesh`))
      (`SceneComponent.SetRelativeScale3D` _box (`self.GrabScale`))
      (`SceneComponent.K2_SetRelativeLocation` _box (`self.GrabLoc`) false false)
      (for _index (range (`PrimitiveComponent.GetNumMaterials` _cube))
        (`PrimitiveComponent.SetMaterial` _cube _index null)))
    (:`then_1`
      (if (`self.Randomness`)
        (`SceneComponent.SetWorldScale3D` _cube_2 (`KismetMathLibrary.MakeVector` _returnvalue _returnvalue _returnvalue))
        (`SceneComponent.K2_SetWorldRotation` _cube_2 (`KismetMathLibrary.MakeRotator` 0.0 0.0 (`KismetMathLibrary.RandomFloatInRange` -180.0 180.0)) false false)))))