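; BP_BlackHole_Simple is an environment black hole with slow timeline-driven rotation and a randomized disc material.
; On BeginPlay, two slowed timelines yaw the Scene component in world space and Scene1 in relative space, the latter as planet rotation.
; Each Rotate update also re-aims the Sphere's yaw toward the world origin with an offset.
; The construction script gives the Sphere a dynamic M_BlackHole_Disc material with a random scalar.
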(event `self.ReceiveBeginPlay`
  (bind _sphere (`self.Sphere`))
  (bind (_returnvalue_roll _returnvalue_pitch _returnvalue_yaw) (`KismetMathLibrary.BreakRotator` (`KismetMathLibrary.FindLookAtRotation` (`SceneComponent.K2_GetComponentLocation` _sphere) (0.0 0.0 0.0))))
  (`|ExecutionSequence`
    (:`then_0`
      (`TimelineComponent.SetPlayRate` (`self.Rotate`) 0.0005)
      (bind (_direction _rotation) (`Timeline|Rotate` :!via `PlayFromStart`)
        (:`Update`
          (`SceneComponent.K2_SetWorldRotation` (`self.Scene`) (`KismetMathLibrary.MakeRotator` 0.0 0.0 _rotation) false false)
          (`SceneComponent.K2_SetWorldRotation` _sphere (`KismetMathLibrary.MakeRotator` 0.0 0.0 (+ _returnvalue_yaw -90.0)) false false))))
    (:`then_1`
      (`TimelineComponent.SetPlayRate` (`self.PlanetRotate`) 0.00075)
      (bind (_direction_2 _planetrotation) (`Timeline|PlanetRotate` :!via `PlayFromStart`)
        (:`Update`
          (`SceneComponent.K2_SetRelativeRotation` (`self.Scene1`) (`KismetMathLibrary.MakeRotator` 0.0 0.0 _planetrotation) false false))))))

(fn `UserConstructionScript`
  (bind _returnvalue (`KismetMaterialLibrary.CreateDynamicMaterialInstance` "/Game/Materials/M_BlackHole_Disc.M_BlackHole_Disc"))
  (`MaterialInstanceDynamic.SetScalarParameterValue` _returnvalue "Random" (`KismetMathLibrary.RandomFloatInRange` 5.0 25.0))
  (`PrimitiveComponent.SetMaterial` (`self.Sphere`) 3 _returnvalue))