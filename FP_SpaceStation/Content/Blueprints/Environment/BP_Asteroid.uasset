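; BP_Asteroid is an environment actor for an asteroid that moves and turns over a randomized duration.
; The construction script rolls a yaw amount, travel time and non-uniform mesh scale, while travel distance is effectively fixed.
; On BeginPlay, the Movement timeline plays at the inverse of that time.
; Its track drives both mesh offset along local X and actor yaw, so the mesh traces a spiral around the actor origin.
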(event `self.ReceiveBeginPlay`
  (`TimelineComponent.SetPlayRate` (`self.Movement`) (/ 1.0 (`self.Time`)))
  (bind (_direction _movement) (`Timeline|Movement`)
    (:`Update`
      (`SceneComponent.K2_SetRelativeLocation` (`self.StaticMesh`) (`KismetMathLibrary.MakeVector` (* _movement (`self.Dist`))) false false)
      (`self.K2_SetActorRotation` (`KismetMathLibrary.MakeRotator` 0.0 0.0 (* _movement (`self.Rot`)))))))

(fn `UserConstructionScript`
  (bind _returnvalue (`KismetMathLibrary.RandomFloatInRange` 1.0 10.0))
  (set `self.Dist` (`KismetMathLibrary.RandomFloatInRange` 160000.0 160000.0))
  (set `self.Rot` (`KismetMathLibrary.RandomFloatInRange` -1000.0 -360.0))
  (set `self.Time` (`KismetMathLibrary.RandomFloatInRange` 25.0 120.0))
  (`SceneComponent.SetWorldScale3D` (`self.StaticMesh`) (`KismetMathLibrary.MakeVector` _returnvalue _returnvalue _returnvalue)))