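; BP_Guitar is a breakable guitar prop that smashes once when hit or swung hard enough.
; A CustomHit event with sufficient force, or a Box1 overlap while the Cube mesh moves fast, triggers the same break.
; Breaking swaps the mesh to the guitar neck, spawns BP_Guitar_Smash at its transform and plays a smash sound.
; The construction script sizes and positions a separate Box from grab scale and location variables.
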(event `self.CustomHit`
  (params (Force :type "Float (single-precision)"))
  (bind _returnvalue (`self.GetTransform`))
  (if (`self.Broken`)
    _
    (elif (>= Force 300.0)
      (set `self.Broken` true :!label _label)
      (`StaticMeshComponent.SetStaticMesh` (`self.Cube`) "/Game/Geometry/FBX_Guitar_Neck.FBX_Guitar_Neck")
      (`|SpawnActorFromClass` "/Game/Blueprints/BP_Guitar_Smash.BP_Guitar_Smash_C" _returnvalue "Undefined" "OverrideRootScale" null null)
      (`GameplayStatics.PlaySoundAtLocation` "/Game/Audio/WAV_GuitarSmash.WAV_GuitarSmash" (.location _returnvalue) (struct) 2.0 1.0 0.0 "/Game/Audio/BasicAttenuation.BasicAttenuation" null null))))

(event `self.Box1.OnComponentBeginOverlap`
  (params (OverlappedComponent :type "PrimitiveComponent Object Reference") (OtherActor :type "Actor Object Reference") (OtherComp :type "PrimitiveComponent Object Reference") (OtherBodyIndex :type Integer) (bFromSweep :type Boolean) (SweepResult :type "HitResult Structure (by ref)"))
  (if (not (`self.Broken`))
    (bind _returnvalue (`PrimitiveComponent.GetPhysicsLinearVelocity` (`self.Cube`) "None"))
    (if (>= (`KismetMathLibrary.VSize` _returnvalue) 600.0)
      (goto _label))))

(fn `UserConstructionScript`
  (bind _box (`self.Box`))
  (`SceneComponent.SetRelativeScale3D` _box (`self.GrabScale`))
  (`SceneComponent.K2_SetRelativeLocation` _box (`self.GrabLoc`) false false))