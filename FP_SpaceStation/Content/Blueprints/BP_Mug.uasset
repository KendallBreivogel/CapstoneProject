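; BP_Mug is a breakable mug actor that shatters when hit hard enough.
; Its CustomHit event checks the incoming force against a fixed threshold, with a Broken flag guarding against repeat triggers.
; On breaking it spawns BP_Mug_Smash at its transform, plays a glass smash sound and destroys itself.
; The construction script sizes and positions the Box component from the GrabScale and GrabLoc variables.
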(event `self.CustomHit`
  (params (Force :type "Float (single-precision)"))
  (bind _returnvalue (`self.GetTransform`))
  (if (`self.Broken`)
    _
    (elif (>= Force 150.0)
      (set `self.Broken` true)
      (`|SpawnActorFromClass` "/Game/Blueprints/BP_Mug_Smash.BP_Mug_Smash_C" _returnvalue "Undefined" "OverrideRootScale" null null)
      (`GameplayStatics.PlaySoundAtLocation` "/Game/Audio/WAV_GlassSmash.WAV_GlassSmash" (.location _returnvalue) (struct) 2.0 1.0 0.0 "/Game/Audio/BasicAttenuation.BasicAttenuation" null null)
      (`self.K2_DestroyActor`))))

(fn `UserConstructionScript`
  (bind _box (`self.Box`))
  (`SceneComponent.SetRelativeScale3D` _box (`self.GrabScale`))
  (`SceneComponent.K2_SetRelativeLocation` _box (`self.GrabLoc`) false false))