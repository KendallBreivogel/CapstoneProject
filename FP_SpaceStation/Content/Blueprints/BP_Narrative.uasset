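; BP_Narrative drives the linear story of a VR space station scene, playing AI voice lines and showing the current task.
; BeginPlay plays timed intro speech, caches the motion controller pawn and shows the first task.
; Incoming narrative events advance the sequence only when they match the next expected event, triggering delayed speech, HUD updates and a one-off station power restore.
; Task text types out character by character through a recursive delayed write.
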(event `self.ReceiveBeginPlay`
  (add `self.NarrativeEvent` (delegate `ForwardNarrative`))
  (`KismetSystemLibrary.Delay` 5.0)
  (`/Game/Blueprints/BP_SpaceStation.PlaySoundThroughSpeakers` (`self.SpaceStation`) "/Game/Audio/WAV_AISpeech_0.WAV_AISpeech_0" false)
  (`KismetSystemLibrary.Delay` 19.0)
  (`/Game/Blueprints/BP_SpaceStation.PlaySoundThroughSpeakers` (`self.SpaceStation`) "/Game/Audio/WAV_AISpeech_1.WAV_AISpeech_1" false)
  (bind _asmotion_controller_pawn (cast `/Game/Blueprints/CharacterBPs/VirtualRealityBP/Blueprints/MotionControllerPawn` (`GameplayStatics.GetPlayerPawn` 0)))
  (set `self.Pawn` _asmotion_controller_pawn)
  (`KismetSystemLibrary.Delay` 14.0)
  (`self.UpdatePlayerHUD`))

(event `ForwardNarrative` :!signature `self.NarrativeEvent`
  (params (EventName :type String))
  (if (`KismetStringLibrary.EqualEqual_StrStr` EventName (`|GetArrayItem` (`self.DesiredEvents`) (`self.NarrativeLoc`)))
    (bind _result (`/Engine/EditorBlueprintResources/StandardMacros.IncrementInt` (`self.NarrativeLoc`))
      (:`  `
        (`|ExecutionSequence`
          (:`then_0`
            (`KismetSystemLibrary.Delay` (`|GetArrayItem` (`self.Delays`) _result))
            (`/Game/Blueprints/BP_SpaceStation.PlaySoundThroughSpeakers` (`self.SpaceStation`) (`|GetArrayItem` (`self.AISpeech`) _result) false)
            (`self.UpdatePlayerHUD`))
          (:`then_1`
            (switch `int` _result
              (:`8`
                (`/Game/Blueprints/BP_SpaceStation.RestorePower` (`self.SpaceStation`))))))))))

(event `UpdatePlayerHUD`
  (set `self.TempText` "")
  (set `self.WriteNum` 0)
  (`self.WriteText`))

(event `WriteText`
  (bind _pawn (`self.Pawn`))
  (bind _writenum (`self.WriteNum`))
  (bind _output (`|GetArrayItem` (`self.TaskDescriptions`) (`self.NarrativeLoc`)))
  (bind _output_get (set `self.TempText` (`KismetStringLibrary.Concat_StrStr` (`self.TempText`) (`KismetStringLibrary.GetSubstring` _output (`self.WriteNum`)))))
  (if (`KismetSystemLibrary.IsValid` _pawn)
    (`TextBlock.SetText` (`/Game/Blueprints/Widgets/W_VRCharacter.Task` (`/Game/Blueprints/CharacterBPs/VirtualRealityBP/Blueprints/MotionControllerPawn.HUD` _pawn)) (`KismetTextLibrary.Conv_StringToText` _output_get))
    (`/Engine/EditorBlueprintResources/StandardMacros.IncrementInt` _writenum
      (:`  `
        (`KismetSystemLibrary.Delay` 0.03)
        (if (not (>= _writenum (`KismetStringLibrary.Len` _output)))
          (`self.WriteText`))))))

(fn `UserConstructionScript`)