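; BP_Record is a grabbable record that works with BP_RecordPlayer.
; Its construction script sets the cube component's mesh and physics, scales and centres the grab box, then applies an optional material to one slot or clears all overrides.
; On PickupTrigger it detaches, keeping its world transform, and stops the first record player found if this is that player's current record.
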(event `self.pickupTrigger`
  (`self.K2_DetachFromActor` "KeepWorld" "KeepWorld" "KeepWorld")
  (bind _outactors (`GameplayStatics.GetAllActorsOfClass` "/Game/Blueprints/StationComponents/BP_RecordPlayer.BP_RecordPlayer_C"))
  (bind _output (`|GetArrayItem` _outactors))
  (bind _currentrecord (`/Game/Blueprints/StationComponents/BP_RecordPlayer.CurrentRecord` _output))
  (if (`KismetSystemLibrary.IsValid` _currentrecord)
    (if (== _currentrecord self)
      (`/Game/Blueprints/StationComponents/BP_RecordPlayer.Stop` _output))))

(fn `UserConstructionScript`
  (bind _cube (`self.Cube`))
  (bind _box (`self.Box`))
  (`PrimitiveComponent.SetSimulatePhysics` (`self.Cube`) (`self.SimulatePhysics`))
  (`StaticMeshComponent.SetStaticMesh` (`self.Cube`) (`self.Mesh`))
  (`SceneComponent.SetRelativeScale3D` _box (`self.GrabScale`))
  (`SceneComponent.K2_SetRelativeLocation` _box (0.0 0.0 0.0) false false)
  (if (`self.UseNewMaterial`)
    (`PrimitiveComponent.SetMaterial` (`self.Cube`) (`self.MatSlot`) (`self.Material`))
    (else
      (for _index (range (`PrimitiveComponent.GetNumMaterials` _cube))
        (`PrimitiveComponent.SetMaterial` _cube _index null)))))