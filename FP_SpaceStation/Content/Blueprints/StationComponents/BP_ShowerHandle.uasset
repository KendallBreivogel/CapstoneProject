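; Rotating shower handle that controls either the temperature or the flow rate of a BP_Shower.
; BeginPlay applies an optional starting roll to the pullable object.
; Update maps that roll to an inverted normalized value, sends it to UpdateTemp or UpdateRate based on IsTempHandle, and debug-prints it.
; When no valid shower is cached, Update instead grabs the first BP_Shower in the level.
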(event `self.ReceiveBeginPlay`
  (bind _startingrot (`self.StartingRot`))
  (if (!= _startingrot 0.0)
    (`SceneComponent.K2_SetRelativeRotation` (`self.PullableObj`) (`KismetMathLibrary.MakeRotator` _startingrot) false false)))

(event `FindShower`
  (bind _outactors (`GameplayStatics.GetAllActorsOfClass` "/Game/Blueprints/StationComponents/BP_Shower.BP_Shower_C"))
  (set `self.Shower` (`|GetArrayItem` _outactors)))

(event `self.Update`
  (bind _shower (`self.Shower`))
  (bind _relativerotation_roll (`KismetMathLibrary.BreakRotator` (`SceneComponent.RelativeRotation` (`self.PullableObj`))))
  (bind _returnvalue (- 1.0 (+ (/ _relativerotation_roll 180.0) 0.5)))
  (if (`KismetSystemLibrary.IsValid` (`self.Shower`))
    (if (`self.IsTempHandle`)
      (`/Game/Blueprints/StationComponents/BP_Shower.UpdateTemp` _shower _returnvalue)
      (else
        (`/Game/Blueprints/StationComponents/BP_Shower.UpdateRate` _shower _returnvalue)))
    (`KismetSystemLibrary.PrintString` (`KismetStringLibrary.Conv_DoubleToString` _returnvalue))
    (else
      (`self.FindShower`))))

(fn `UserConstructionScript`)