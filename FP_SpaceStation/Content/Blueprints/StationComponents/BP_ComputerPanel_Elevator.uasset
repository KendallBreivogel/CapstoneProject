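; BP_ComputerPanel_Elevator is a VR touchscreen computer panel that controls its parent elevator actor.
; On BeginPlay it switches its widget to the elevator screen and adds the parent BP_Elevator to its receiver array.
; A motion controller entering the Box triggers a touchscreen press if its widget interaction is over an interactable widget.
; ButtonPress forwards an action number to the receiver at the given index.
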(event `self.ReceiveBeginPlay`
  (bind _asw_computer_panel_template (cast `/Game/Blueprints/Widgets/W_ComputerPanel_Template` (`WidgetComponent.GetUserWidgetObject` (`self.Widget`))))
  (`/Game/Blueprints/Widgets/W_ComputerPanel_Template.ShowElevatorScreen` _asw_computer_panel_template)
  (bind _asbp_elevator (cast `/Game/Blueprints/StationComponents/BP_Elevator` (`self.GetParentActor`)))
  (bind _output_get (set `self.Elevator` _asbp_elevator))
  (`KismetArrayLibrary.Array_Add` (`self.Reciever`) _output_get))

(event `self.Box.OnComponentBeginOverlap`
  (params (OverlappedComponent :type "PrimitiveComponent Object Reference") (OtherActor :type "Actor Object Reference") (OtherComp :type "PrimitiveComponent Object Reference") (OtherBodyIndex :type Integer) (bFromSweep :type Boolean) (SweepResult :type "HitResult Structure (by ref)"))
  (bind _asbp_motion_controller (cast `/Game/Blueprints/CharacterBPs/VirtualRealityBP/Blueprints/BP_MotionController` OtherActor))
  (if (`WidgetInteractionComponent.IsOverInteractableWidget` (`/Game/Blueprints/CharacterBPs/VirtualRealityBP/Blueprints/BP_MotionController.WidgetInteraction` _asbp_motion_controller))
    (`/Game/Blueprints/CharacterBPs/VirtualRealityBP/Blueprints/BP_MotionController.PressTouchscreen` _asbp_motion_controller)))

(fn `ButtonPress`
  (params (RecieverNum :type Integer) (ActionNum :type Integer))
  (`/Game/Blueprints/StationComponents/Templates/BP_Reciever.Action` (`|GetArrayItem` (`self.Reciever`) RecieverNum) ActionNum))

(fn `UserConstructionScript`)