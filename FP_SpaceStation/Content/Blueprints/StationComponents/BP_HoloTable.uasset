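; BP_HoloTable is a station hologram table that switches its projection between Station, Orbit and Starfield modes.
; The construction script caches and hides a child-actor BP_Hologram, which SetActivated shows after a short delay or hides immediately.
; SwitchHoloMode clears overlays, calls the hologram's transition for the current and requested pair, then stores the mode.
; Tick spins the projector ring, while a laser-pointer trace to the hologram sits unconnected.
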(event `SwitchHoloMode`
  (params (newHoloMode :type "/Game/Blueprints/HoloMode Enum" :default "NewEnumerator0"))
  (bind _holomode (`self.holoMode`))
  (bind _hologram (`self.Hologram`))
  (bind _hologram_2 (`self.Hologram`))
  (bind _hologram_3 (`self.Hologram`))
  (`/Game/Blueprints/StationComponents/BP_Hologram.DisableOverlays` (`self.Hologram`))
  (switch `/Game/Blueprints/HoloMode` newHoloMode
    (:`NewEnumerator0`
      (switch `/Game/Blueprints/HoloMode` _holomode
        (:`NewEnumerator1`
          (`/Game/Blueprints/StationComponents/BP_Hologram.Switch_OrbitToStation` _hologram_2))
        (:`NewEnumerator2`
          (`/Game/Blueprints/StationComponents/BP_Hologram.Switch_StarfieldToStation` _hologram_2)))
      (set `self.holoMode` "NewEnumerator0"))
    (:`NewEnumerator1`
      (switch `/Game/Blueprints/HoloMode` _holomode
        (:`NewEnumerator0`
          (`/Game/Blueprints/StationComponents/BP_Hologram.Switch_StationToOrbit` _hologram))
        (:`NewEnumerator2`
          (`/Game/Blueprints/StationComponents/BP_Hologram.Switch_StarfieldToOrbit` _hologram)))
      (set `self.holoMode` "NewEnumerator1"))
    (:`NewEnumerator2`
      (switch `/Game/Blueprints/HoloMode` _holomode
        (:`NewEnumerator0`
          (`/Game/Blueprints/StationComponents/BP_Hologram.Switch_StationToStarfield` _hologram_3))
        (:`NewEnumerator1`
          (`/Game/Blueprints/StationComponents/BP_Hologram.Switch_OrbitToStarfield` _hologram_3)))
      (set `self.holoMode` "NewEnumerator2"))))

(event `self.ReceiveBeginPlay`)

(event `SetActivated`
  (params (Active :type Boolean))
  (bind _hologram (`self.Hologram`))
  (if Active
    (`KismetSystemLibrary.Delay` 0.2)
    (`self.SetActorHiddenInGame` _hologram false)
    (else
      (`self.SetActorHiddenInGame` _hologram true))))

(event `self.ReceiveTick`
  (params (DeltaSeconds :type "Float (single-precision)"))
  (`SceneComponent.K2_AddLocalRotation` (`self.FBX_HoloTable_ProjectorRing`) (struct :`Yaw` 0.01) false false))

(fn `UserConstructionScript`
  (bind _asbp_hologram (cast `/Game/Blueprints/StationComponents/BP_Hologram` (`ChildActorComponent.ChildActor` (`self.BP_Hologram`))))
  (set `self.Hologram` _asbp_hologram)
  (`self.SetActorHiddenInGame` (`self.Hologram`) true))