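; Station component Blueprint for a set of misters that can be switched on and off.
; BeginPlay sets the SpawnRate parameter on eight mist particle components.
; StartMisting and StopMisting set the On flag, activate or deactivate all eight emitters without resetting them, and fade four audio components in or out alongside them.
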(event `self.ReceiveBeginPlay`
  (`ParticleSystemComponent.SetFloatParameter` (`self.Mist_1`) "SpawnRate" 1.0)
  (`ParticleSystemComponent.SetFloatParameter` (`self.Mist_2`) "SpawnRate" 1.0)
  (`ParticleSystemComponent.SetFloatParameter` (`self.Mist_3`) "SpawnRate" 1.0)
  (`ParticleSystemComponent.SetFloatParameter` (`self.Mist_4`) "SpawnRate" 1.0)
  (`ParticleSystemComponent.SetFloatParameter` (`self.Mist_5`) "SpawnRate" 1.0)
  (`ParticleSystemComponent.SetFloatParameter` (`self.Mist_6`) "SpawnRate" 1.0)
  (`ParticleSystemComponent.SetFloatParameter` (`self.Mist_7`) "SpawnRate" 1.0)
  (`ParticleSystemComponent.SetFloatParameter` (`self.Mist_8`) "SpawnRate" 1.0))

(event `StartMisting`
  (set `self.On` true)
  (`ActorComponent.SetActive` (`self.Mist_1`) true false)
  (`ActorComponent.SetActive` (`self.Mist_2`) true false)
  (`ActorComponent.SetActive` (`self.Mist_3`) true false)
  (`ActorComponent.SetActive` (`self.Mist_4`) true false)
  (`ActorComponent.SetActive` (`self.Mist_5`) true false)
  (`ActorComponent.SetActive` (`self.Mist_6`) true false)
  (`ActorComponent.SetActive` (`self.Mist_7`) true false)
  (`ActorComponent.SetActive` (`self.Mist_8`) true false)
  (`AudioComponent.FadeIn` (`self.WAV_Misters`) 3.0 0.3 0.0)
  (`AudioComponent.FadeIn` (`self.Audio`) 3.0 0.3 0.0)
  (`AudioComponent.FadeIn` (`self.Audio1`) 3.0 0.3 0.0)
  (`AudioComponent.FadeIn` (`self.Audio2`) 3.0 0.3 0.0))

(event `StopMisting`
  (set `self.On` false)
  (`ActorComponent.SetActive` (`self.Mist_1`) false false)
  (`ActorComponent.SetActive` (`self.Mist_2`) false false)
  (`ActorComponent.SetActive` (`self.Mist_3`) false false)
  (`ActorComponent.SetActive` (`self.Mist_4`) false false)
  (`ActorComponent.SetActive` (`self.Mist_5`) false false)
  (`ActorComponent.SetActive` (`self.Mist_6`) false false)
  (`ActorComponent.SetActive` (`self.Mist_7`) false false)
  (`ActorComponent.SetActive` (`self.Mist_8`) false false)
  (`AudioComponent.FadeOut` (`self.WAV_Misters`) 3.0 0.0)
  (`AudioComponent.FadeOut` (`self.Audio`) 3.0 0.0)
  (`AudioComponent.FadeOut` (`self.Audio1`) 3.0 0.0)
  (`AudioComponent.FadeOut` (`self.Audio2`) 3.0 0.0))

(fn `UserConstructionScript`)