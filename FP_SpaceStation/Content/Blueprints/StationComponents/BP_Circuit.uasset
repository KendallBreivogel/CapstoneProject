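; BP_Circuit is a station circuit chip that can be flagged as broken and reports when a broken one is dropped.
; The construction script gives broken chips a flashing red emissive material via a dynamic instance.
; On CustomDrop, a broken chip decrements the bad-chip count on its parent BP_StandIn_ChipDrawer, then fires the "badChipRemoved" event on the first BP_Narrative actor found.
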(event `self.CustomDrop`
  (if (`self.IsBroken`)
    (bind _asbp_stand_in_chip_drawer (cast `/Game/Blueprints/StationComponents/BP_StandIn_ChipDrawer` (`self.GetParentActor`)))
    (`/Game/Blueprints/StationComponents/BP_StandIn_ChipDrawer.DecrementBadChipNum` _asbp_stand_in_chip_drawer)
    (bind _outactors (`GameplayStatics.GetAllActorsOfClass` "/Game/Blueprints/BP_Narrative.BP_Narrative_C"))
    (`/Game/Blueprints/BP_Narrative.NarrativeEvent` (`|GetArrayItem` _outactors) "badChipRemoved")))

(fn `UserConstructionScript`
  (if (`self.IsBroken`)
    (bind _returnvalue (`KismetMaterialLibrary.CreateDynamicMaterialInstance` "/Game/Materials/MI_Emissive_Red_Flashing.MI_Emissive_Red_Flashing"))
    (`PrimitiveComponent.SetMaterialByName` (`self.Cube`) "M_Emissive" _returnvalue)))