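; BP_PowerSwitch is a station power switch that toggles IsOn from the position of a pullable handle.
; Update compares actor and handle world Y against opposite thresholds for hysteresis, with InverseSwitch flipping the direction.
; State changes set the emissive color of a dynamic material created in construction, amber for on and black for off.
; When IsNarrativeObj is set, switching on fires the "powerReset" event on the first BP_Narrative found.
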(event `self.ReceiveBeginPlay`
  (`SceneComponent.K2_SetRelativeLocation` (`self.PullableObj`) (0.0 3.9 0.0) false false))

(event `self.Update`
  (bind (_returnvalue_x _returnvalue_y) (`KismetMathLibrary.BreakVector` (`self.K2_GetActorLocation`)))
  (bind (_returnvalue_x_2 _returnvalue_y_2) (`KismetMathLibrary.BreakVector` (`SceneComponent.K2_GetComponentLocation` (`self.PullableObj`))))
  (bind _returnvalue (- _returnvalue_y _returnvalue_y_2))
  (bind _returnvalue_2 (<= _returnvalue -3.85))
  (bind _returnvalue_3 (>= _returnvalue 3.85))
  (if (`self.InverseSwitch`)
    (if (`self.IsOn`)
      (if _returnvalue_3
        (set `self.IsOn` false)
        (`MaterialInstanceDynamic.SetVectorParameterValue` (`self.Mat`) "EmissiveColor" (struct :`A` 1.0)))
      (elif _returnvalue_2
        (set `self.IsOn` true)
        (`MaterialInstanceDynamic.SetVectorParameterValue` (`self.Mat`) "EmissiveColor" (struct :`R` 1.0 :`G` 0.631373 :`A` 1.0))
        (if (`self.isNarrativeObj`)
          (bind _outactors (`GameplayStatics.GetAllActorsOfClass` "/Game/Blueprints/BP_Narrative.BP_Narrative_C"))
          (`/Game/Blueprints/BP_Narrative.NarrativeEvent` (`|GetArrayItem` _outactors) "powerReset"))))
    (elif (`self.IsOn`)
      (if _returnvalue_2
        (set `self.IsOn` false)
        (`MaterialInstanceDynamic.SetVectorParameterValue` (`self.Mat`) "EmissiveColor" (struct :`A` 1.0)))
      (elif _returnvalue_3
        (set `self.IsOn` true)
        (`MaterialInstanceDynamic.SetVectorParameterValue` (`self.Mat`) "EmissiveColor" (struct :`R` 1.0 :`G` 0.631373 :`A` 1.0))
        (if (`self.isNarrativeObj`)
          (bind _outactors_2 (`GameplayStatics.GetAllActorsOfClass` "/Game/Blueprints/BP_Narrative.BP_Narrative_C"))
          (`/Game/Blueprints/BP_Narrative.NarrativeEvent` (`|GetArrayItem` _outactors_2) "powerReset"))))))

(fn `UserConstructionScript`
  (bind _returnvalue (`KismetMaterialLibrary.CreateDynamicMaterialInstance` "/Game/Materials/M_Emissive_Master.M_Emissive_Master"))
  (bind _output_get (set `self.Mat` _returnvalue))
  (`PrimitiveComponent.SetMaterialByName` (`self.Cube`) "M_Emissive" _output_get)
  (`MaterialInstanceDynamic.SetVectorParameterValue` (`self.Mat`) "EmissiveColor" (struct :`R` 1.0 :`G` 0.631373 :`A` 1.0)))