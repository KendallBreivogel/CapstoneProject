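; BP_Oven is an oven station component that glows orange while cookware is inside its Box volume.
; The construction script assigns a dynamic emissive material to the oven mesh's emissive slot, starting at zero brightness.
; Cookware overlaps play the OvenGlow timeline to scale emissive brightness, and end overlaps reverse it.
; Only the visual glow is handled here, with no cooking logic.
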(event `self.Box.OnComponentBeginOverlap`
  (params (OverlappedComponent :type "PrimitiveComponent Object Reference") (OtherActor :type "Actor Object Reference") (OtherComp :type "PrimitiveComponent Object Reference") (OtherBodyIndex :type Integer) (bFromSweep :type Boolean) (SweepResult :type "HitResult Structure (by ref)"))
  (cast `/Game/Blueprints/BP_Cookware` OtherActor)
  (bind (_direction _glow) (`Timeline|OvenGlow` :!label _label)
    (:`Update`
      (`MaterialInstanceDynamic.SetScalarParameterValue` (`self.GlowMat`) "EmissiveBrightness" (* _glow 100.0)))))

(event `self.Box.OnComponentEndOverlap`
  (params (OverlappedComponent :type "PrimitiveComponent Object Reference") (OtherActor :type "Actor Object Reference") (OtherComp :type "PrimitiveComponent Object Reference") (OtherBodyIndex :type Integer))
  (cast `/Game/Blueprints/BP_Cookware` OtherActor)
  (goto _label :!via `Reverse`))

(fn `UserConstructionScript`
  (bind _glowmat (`self.GlowMat`))
  (bind _returnvalue (`KismetMaterialLibrary.CreateDynamicMaterialInstance` "/Game/Materials/M_Emissive_Master.M_Emissive_Master"))
  (bind _output_get (set `self.GlowMat` _returnvalue))
  (`MaterialInstanceDynamic.SetVectorParameterValue` _output_get "EmissiveColor" (struct :`R` 1.0 :`G` 0.497933 :`A` 1.0))
  (`MaterialInstanceDynamic.SetVectorParameterValue` _glowmat "EmissiveColor" (struct :`R` 1.0 :`G` 0.497933 :`A` 1.0))
  (`MaterialInstanceDynamic.SetScalarParameterValue` _glowmat "EmissiveBrightness" 0.0)
  (`PrimitiveComponent.SetMaterialByName` (`self.FBX_Kitchenette_Oven`) "EmissiveMaster" _glowmat))