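; BP_UnlockHandle is a physics-simulated pullable handle that controls one of the two-state locks on its parent BP_Sensor_ChipDrawer, chosen by IsLock1.
; BeginPlay applies an optional starting yaw to the handle.
; On CustomDrop, it reports unlocked or locked to the drawer depending on whether its yaw sits within a negative quarter turn.
; The drawer reference resolves lazily, so a drop without one only caches it and prints failure.
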(event `self.ReceiveBeginPlay`
  (bind _startingrot (`self.StartingRot`))
  (if (!= _startingrot 0.0)
    (`SceneComponent.K2_SetRelativeRotation` (`self.PullableObj`) (`KismetMathLibrary.MakeRotator` 0.0 0.0 _startingrot) false false)))

(event `FindDrawer`
  (bind _asbp_sensor_chip_drawer (cast `/Game/Blueprints/StationComponents/BP_Sensor_ChipDrawer` (`self.GetParentActor`)))
  (set `self.Drawer` _asbp_sensor_chip_drawer))

(event `/Game/Blueprints/StationComponents/Templates/BP_Grabbable.CustomDrop`
  (bind _drawer (`self.Drawer`))
  (bind _islock1 (`self.IsLock1`))
  (bind (_relativerotation_roll _relativerotation_pitch _relativerotation_yaw) (`KismetMathLibrary.BreakRotator` (`SceneComponent.RelativeRotation` (`self.PullableObj`))))
  (if (`KismetSystemLibrary.IsValid` (`self.Drawer`))
    (if (and (< _relativerotation_yaw 0.0) (>= _relativerotation_yaw -90.0))
      (`/Game/Blueprints/StationComponents/BP_Sensor_ChipDrawer.UpdateLocks` _drawer _islock1 true)
      (`KismetSystemLibrary.PrintString` "One unlocked!")
      (else
        (`/Game/Blueprints/StationComponents/BP_Sensor_ChipDrawer.UpdateLocks` _drawer _islock1 false)
        (`KismetSystemLibrary.PrintString` "Failure!" :!label _label)))
    (else
      (`self.FindDrawer`)
      (goto _label))))

(fn `UserConstructionScript`
  (`PrimitiveComponent.SetSimulatePhysics` (`self.PullableObj`) true))