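; Sliding toilet door for a station component that opens on interaction and closes itself once a pawn leaves its trigger box.
; A single timeline slides the cube along its local X axis, playing forward to open and in reverse to close, with interaction locked until it finishes.
; Leaving the box while the door is open starts a short close timer, which re-entering cancels.
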(event `Close`
  (set `self.CanInteract` false)
  (set `self.IsOpen` false)
  (bind (_direction _doorpos) (`Timeline|DoorMotion` :!via `Reverse` :!label _label)
    (:`Update`
      (`SceneComponent.K2_SetRelativeLocation` (`self.Cube`) (`KismetMathLibrary.MakeVector` (* _doorpos -100.0)) false false))
    (:`Finished`
      (set `self.CanInteract` true))))

(event `Open`
  (set `self.CanInteract` false :!label _label_2)
  (set `self.IsOpen` true)
  (goto _label))

(event `self.InteractPC`
  (if (`self.CanInteract`) :!label _label_3
    (if (not (`self.IsOpen`))
      (goto _label_2))))

(event `self.Interact`
  (goto _label_3))

(event `self.Box.OnComponentEndOverlap`
  (params (OverlappedComponent :type "PrimitiveComponent Object Reference") (OtherActor :type "Actor Object Reference") (OtherComp :type "PrimitiveComponent Object Reference") (OtherBodyIndex :type Integer))
  (cast `Pawn` OtherActor)
  (if (`self.IsOpen`)
    (bind _returnvalue (`KismetSystemLibrary.K2_SetTimerDelegate` (delegate `Close`) 1.5))))

(event `self.Box.OnComponentBeginOverlap`
  (params (OverlappedComponent :type "PrimitiveComponent Object Reference") (OtherActor :type "Actor Object Reference") (OtherComp :type "PrimitiveComponent Object Reference") (OtherBodyIndex :type Integer) (bFromSweep :type Boolean) (SweepResult :type "HitResult Structure (by ref)"))
  (cast `Pawn` OtherActor)
  (if (`self.IsOpen`)
    (`KismetSystemLibrary.K2_ClearAndInvalidateTimerHandle` (stale `self.Box.OnComponentEndOverlap` _returnvalue))))

(fn `UserConstructionScript`)