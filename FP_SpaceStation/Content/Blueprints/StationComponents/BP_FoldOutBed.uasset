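; Fold-out bed station component that can be pulled by physics grab and shows impressions in its fabric where objects overlap it.
; Pickup makes a physics handle follow the grabbing component on a timer; Drop releases it and snaps the bed to zero rotation below a small roll angle.
; A sensor tracks up to three overlapping actors, including motion controllers, while a looping timer lerps their coordinates into dynamic material parameters.
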(event `CustomEvent`
  (`PhysicsHandleComponent.SetTargetLocation` (`self.PhysicsHandle_Handle`) (`SceneComponent.K2_GetComponentLocation` (`self.AttachedComponent`))))

(event `TrackObject`
  (bind _trackedobjectnum (`self.TrackedObjectNum`))
  (`|ExecutionSequence`
    (:`then_0`
      (bind _parametervalue (`self.GetImpressionParameter` (`self.TrackedObject1`) false "ImpressionLocation1"))
      (`MaterialInstanceDynamic.SetVectorParameterValue` (`self.ImpressiveFabric`) "ImpressionLocation1" _parametervalue))
    (:`then_1`
      (if (> _trackedobjectnum 1)
        (bind _parametervalue_2 (`self.GetImpressionParameter` (`self.TrackedObject2`) false "ImpressionLocation2"))
        (`MaterialInstanceDynamic.SetVectorParameterValue` (`self.ImpressiveFabric`) "ImpressionLocation2" _parametervalue_2)))
    (:`then_2`
      (if (> _trackedobjectnum 2)
        (bind _parametervalue_3 (`self.GetImpressionParameter` (`self.TrackedObject3`) false "ImpressionLocation3"))
        (`MaterialInstanceDynamic.SetVectorParameterValue` (`self.ImpressiveFabric`) "ImpressionLocation3" _parametervalue_3)))))

(event `/Game/Blueprints/CharacterBPs/VirtualRealityBP/Blueprints/PickupActorInterface.Pickup`
  (params (AttachTo :type "SceneComponent Object Reference"))
  (bind _pullableobj (`self.PullableObj`))
  (bind _output_get (set `self.AttachedComponent` AttachTo))
  (`PhysicsHandleComponent.GrabComponentAtLocation` (`self.PhysicsHandle_Handle`) _pullableobj "None" (`SceneComponent.K2_GetComponentLocation` _output_get))
  (`PrimitiveComponent.SetSimulatePhysics` _pullableobj true)
  (bind _returnvalue (`KismetSystemLibrary.K2_SetTimerDelegate` (delegate `CustomEvent`) 0.03 true)))

(event `/Game/Blueprints/CharacterBPs/VirtualRealityBP/Blueprints/PickupActorInterface.Drop`
  (bind _pullableobj (`self.PullableObj`))
  (bind _relativerotation_roll (`KismetMathLibrary.BreakRotator` (`SceneComponent.RelativeRotation` (`self.PullableObj`))))
  (`PhysicsHandleComponent.ReleaseComponent` (`self.PhysicsHandle_Handle`))
  (set `self.AttachedComponent` null)
  (`KismetSystemLibrary.K2_ClearAndInvalidateTimerHandle` (stale `/Game/Blueprints/CharacterBPs/VirtualRealityBP/Blueprints/PickupActorInterface.Pickup` _returnvalue))
  (if (< _relativerotation_roll 4.0)
    (`SceneComponent.K2_SetRelativeRotation` :`self` _pullableobj)
    (`PrimitiveComponent.SetSimulatePhysics` _pullableobj false)))

(event `self.ImpressionSensor.OnComponentBeginOverlap`
  (params (OverlappedComponent :type "PrimitiveComponent Object Reference") (OtherActor :type "Actor Object Reference") (OtherComp :type "PrimitiveComponent Object Reference") (OtherBodyIndex :type Integer) (bFromSweep :type Boolean) (SweepResult :type "HitResult Structure (by ref)"))
  (bind _impressivefabric (`self.ImpressiveFabric`))
  (switch `int` (`self.TrackedObjectNum`)
    (:`0`
      (set `self.TrackedObject1` OtherActor)
      (set `self.TrackedObjectNum` 1)
      (bind _parametervalue (`self.GetImpressionParameter` (`self.TrackedObject1`) true "ImpressionLocation1"))
      (`MaterialInstanceDynamic.SetVectorParameterValue` _impressivefabric "ImpressionLocation1" _parametervalue)
      (bind _returnvalue (`KismetSystemLibrary.K2_SetTimerDelegate` (delegate `TrackObject`) 0.01 true)))
    (:`1`
      (set `self.TrackedObject2` OtherActor)
      (set `self.TrackedObjectNum` 2)
      (bind _parametervalue_2 (`self.GetImpressionParameter` (`self.TrackedObject2`) true "ImpressionLocation2"))
      (`MaterialInstanceDynamic.SetVectorParameterValue` _impressivefabric "ImpressionLocation2" _parametervalue_2))
    (:`2`
      (set `self.TrackedObject3` OtherActor)
      (set `self.TrackedObjectNum` 3)
      (bind _parametervalue_3 (`self.GetImpressionParameter` (`self.TrackedObject3`) true "ImpressionLocation3"))
      (`MaterialInstanceDynamic.SetVectorParameterValue` _impressivefabric "ImpressionLocation3" _parametervalue_3))))

(event `self.ImpressionSensor.OnComponentEndOverlap`
  (params (OverlappedComponent :type "PrimitiveComponent Object Reference") (OtherActor :type "Actor Object Reference") (OtherComp :type "PrimitiveComponent Object Reference") (OtherBodyIndex :type Integer))
  (bind _trackedobjectnum (`self.TrackedObjectNum`))
  (if (== OtherActor (`self.TrackedObject1`))
    (switch `int` _trackedobjectnum
      (:`1`
        (set `self.TrackedObject1` null)
        (set `self.TrackedObjectNum` 0)
        (`MaterialInstanceDynamic.SetVectorParameterValue` (`self.ImpressiveFabric`) "ImpressionLocation1" (struct :`R` 2.0 :`G` 2.0 :`A` 1.0))
        (`KismetSystemLibrary.K2_ClearAndInvalidateTimerHandle` (stale `self.ImpressionSensor.OnComponentBeginOverlap` _returnvalue)))
      (:`2`
        (if (`KismetSystemLibrary.IsValid` (`self.TrackedObject2`))
          (set `self.TrackedObject1` (`self.TrackedObject2`))
          (set `self.TrackedObject2` null)
          (else
            (set `self.TrackedObject1` (`self.TrackedObject3`))
            (set `self.TrackedObject3` null)))
        (set `self.TrackedObjectNum` 1)
        (`MaterialInstanceDynamic.SetVectorParameterValue` (`self.ImpressiveFabric`) "ImpressionLocation2" (struct :`R` 2.0 :`G` 2.0 :`A` 1.0)))
      (:`3`
        (set `self.TrackedObject1` (`self.TrackedObject3`))
        (set `self.TrackedObject3` null)
        (set `self.TrackedObjectNum` 2)
        (`MaterialInstanceDynamic.SetVectorParameterValue` (`self.ImpressiveFabric`) "ImpressionLocation3" (struct :`R` 2.0 :`G` 2.0 :`A` 1.0))))
    (elif (== OtherActor (`self.TrackedObject2`))
      (switch `int` _trackedobjectnum
        (:`2`
          (set `self.TrackedObject2` null)
          (set `self.TrackedObjectNum` 1)
          (`MaterialInstanceDynamic.SetVectorParameterValue` (`self.ImpressiveFabric`) "ImpressionLocation2" (struct :`R` 2.0 :`G` 2.0 :`A` 1.0)))
        (:`3`
          (set `self.TrackedObject2` (`self.TrackedObject3`))
          (set `self.TrackedObject3` null)
          (set `self.TrackedObjectNum` 2)
          (`MaterialInstanceDynamic.SetVectorParameterValue` (`self.ImpressiveFabric`) "ImpressionLocation3" (struct :`R` 2.0 :`G` 2.0 :`A` 1.0))))
      (elif (== OtherActor (`self.TrackedObject3`))
        (set `self.TrackedObject3` null)
        (set `self.TrackedObjectNum` 2)
        (`MaterialInstanceDynamic.SetVectorParameterValue` (`self.ImpressiveFabric`) "ImpressionLocation3" (struct :`R` 2.0 :`G` 2.0 :`A` 1.0))))))

(fn `GetImpressionParameter`
  (params (TrackedObject :type "Actor Object Reference") (Instant :type Boolean) (parameterName :type Name))
  (returns (ParameterValue :type "LinearColor Structure"))
  (bind _xy (`self.GetCoords` (`self.K2_GetActorLocation` TrackedObject)))
  (bind (_r _g _b) (break `LinearColor` _xy))
  (bind _asbp_motion_controller (cast `/Game/Blueprints/CharacterBPs/VirtualRealityBP/Blueprints/BP_MotionController` TrackedObject)
    (:`then`
      (bind _returnvalue (`MaterialInstanceDynamic.K2_GetVectorParameterValue` (`self.ImpressiveFabric`) parameterName))
      (if Instant
        (bind _xy_2 (`self.GetCoords` (`SceneComponent.K2_GetComponentLocation` (`/Game/Blueprints/CharacterBPs/VirtualRealityBP/Blueprints/BP_MotionController.MotionController` _asbp_motion_controller))))
        (bind (_r_2 _g_2 _b_2) (break `LinearColor` _xy_2))
        (return (make `LinearColor` _r_2 _g_2 (`KismetMathLibrary.Lerp` (`.B` (break `LinearColor` _returnvalue)) _b_2 0.08)))
        (else
          (return (`KismetMathLibrary.LinearColorLerp` _returnvalue _xy_2 0.08)))))
    (:`CastFailed`
      (bind _returnvalue_2 (`MaterialInstanceDynamic.K2_GetVectorParameterValue` (`self.ImpressiveFabric`) parameterName))
      (if Instant
        (return (make `LinearColor` _r _g (`KismetMathLibrary.Lerp` (`.B` (break `LinearColor` _returnvalue_2)) _b 0.08)))
        (else
          (return (`KismetMathLibrary.LinearColorLerp` _returnvalue_2 _xy 0.08)))))))

(fn `UserConstructionScript`
  (bind _returnvalue (`KismetMaterialLibrary.CreateDynamicMaterialInstance` "/Game/Materials/M_ImpressableFabric.M_ImpressableFabric"))
  (bind _output_get (set `self.ImpressiveFabric` _returnvalue))
  (`PrimitiveComponent.SetMaterialByName` (`self.PullableObj`) "impressable" _output_get))