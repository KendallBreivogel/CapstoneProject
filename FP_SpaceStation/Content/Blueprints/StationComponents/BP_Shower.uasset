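; BP_Shower is a station component that drives a shower's water, splash and steam particle effects from a flow rate and a temperature.
; UpdateRate sets the spawn rate of the water drops and splash ripples, derives an On flag from a positive rate, and toggles the steam to match.
; UpdateTemp feeds temperature into the steam spawn rate.
; On BeginPlay it applies a default temperature and keeps steam inactive.
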(event `self.ReceiveBeginPlay`
  (`self.UpdateTemp` 0.5)
  (`ActorComponent.SetActive` (`self.P_Steam_Lit`) false false))

(event `UpdateRate`
  (params (newRate :type "Float (double-precision)"))
  (bind _rate (`self.Rate`))
  (set `self.Rate` newRate)
  (`ParticleSystemComponent.SetFloatParameter` (`self.P_WaterDrops`) "SpawnRate" _rate)
  (`ParticleSystemComponent.SetFloatParameter` (`self.P_Splash_Ripples`) "SpawnRate" _rate)
  (if (> (`self.Rate`) 0.0)
    (set `self.On` true)
    (else
      (set `self.On` false)))
  (`ActorComponent.SetActive` (`self.P_Steam_Lit`) (`self.On`) false))

(event `UpdateTemp`
  (params (newTemp :type "Float (double-precision)"))
  (set `self.Temp` newTemp)
  (`ParticleSystemComponent.SetFloatParameter` (`self.P_Steam_Lit`) "SpawnRate" (`self.Temp`)))

(fn `UserConstructionScript`)