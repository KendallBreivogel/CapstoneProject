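; BP_Module1_Bulkheads is a space station module's bulkheads, which toggle between open and closed.
; The OpenBulkheads timeline's Height track slides the Upper and Lower parts apart vertically and pitches eight ceiling pieces spaced 45 degrees apart in yaw.
; Action plays or reverses the timeline, reporting status to BP_SpaceStation when closing starts and when either movement finishes.
; BeginPlay finds the station and jumps the timeline to match the Open flag.
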(event `self.ReceiveBeginPlay`
  (bind _outactors (`GameplayStatics.GetAllActorsOfClass` "/Game/Blueprints/BP_SpaceStation.BP_SpaceStation_C"))
  (set `self.SpaceStation` (`|GetArrayItem` _outactors))
  (if (`self.Open`)
    (`self.OpenInstant`)
    (else
      (`self.CloseInstant`))))

(event `OpenInstant`
  (`TimelineComponent.SetNewTime` (`self.OpenBulkheads`) 12.0))

(event `CloseInstant`
  (`TimelineComponent.SetNewTime` (`self.OpenBulkheads`) 0.0))

(event `self.Action`
  (params (ActionNum :type Integer))
  (bind _spacestation (`self.SpaceStation`))
  (if (`self.Open`)
    (set `self.Open` false)
    (`/Game/Blueprints/BP_SpaceStation.StatusChange` (`self.SpaceStation`) "NewEnumerator1" false)
    (bind (_direction _height) (`Timeline|OpenBulkheads` :!via `Reverse` :!label _label)
      (:`Update`
        (`SceneComponent.K2_SetRelativeLocation` (`self.Lower`) (`KismetMathLibrary.MakeVector` 0.0 0.0 (* _height -100.0)) false false)
        (`SceneComponent.K2_SetRelativeLocation` (`self.Upper`) (`KismetMathLibrary.MakeVector` 0.0 0.0 (* _height 100.0)) false false)
        (bind _returnvalue (* _height 150.0))
        (`SceneComponent.K2_SetRelativeRotation` (`self.Ceiling1`) (`KismetMathLibrary.MakeRotator` 0.0 _returnvalue) false false)
        (`SceneComponent.K2_SetRelativeRotation` (`self.Ceiling2`) (`KismetMathLibrary.MakeRotator` 0.0 _returnvalue -45.0) false false)
        (`SceneComponent.K2_SetRelativeRotation` (`self.Ceiling3`) (`KismetMathLibrary.MakeRotator` 0.0 _returnvalue -90.0) false false)
        (`SceneComponent.K2_SetRelativeRotation` (`self.Ceiling4`) (`KismetMathLibrary.MakeRotator` 0.0 _returnvalue -135.0) false false)
        (`SceneComponent.K2_SetRelativeRotation` (`self.Ceiling5`) (`KismetMathLibrary.MakeRotator` 0.0 _returnvalue -180.0) false false)
        (`SceneComponent.K2_SetRelativeRotation` (`self.Ceiling6`) (`KismetMathLibrary.MakeRotator` 0.0 _returnvalue -225.0) false false)
        (`SceneComponent.K2_SetRelativeRotation` (`self.Ceiling7`) (`KismetMathLibrary.MakeRotator` 0.0 _returnvalue -270.0) false false)
        (`SceneComponent.K2_SetRelativeRotation` (`self.Ceiling8`) (`KismetMathLibrary.MakeRotator` 0.0 _returnvalue -315.0) false false))
      (:`Finished`
        (if (`self.Open`)
          (`/Game/Blueprints/BP_SpaceStation.StatusChange` _spacestation "NewEnumerator0" false)
          (else
            (`/Game/Blueprints/BP_SpaceStation.StatusChange` _spacestation "NewEnumerator3" false)))))
    (else
      (set `self.Open` true)
      (goto _label))))

(fn `UserConstructionScript`)