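; Record player station component that plays the LP sound of a BP_Record dropped into its trigger box through two placeable speakers.
; The record snaps to the turnpoint, then staggered delays swing the needle in, start a timer-driven spin ramped by timeline, and begin playback.
; When the spin tick finds Speaker1 silent during playback, Stop fades audio, reverses both timelines and clears the timer and state after a delay.
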(event `self.ReceiveBeginPlay`
  (bind _outactors (`GameplayStatics.GetAllActorsOfClass` "/Game/Blueprints/BP_SpaceStation.BP_SpaceStation_C"))
  (set `self.SpaceStation` (`|GetArrayItem` _outactors)))

(event `RotateRecord`
  (`SceneComponent.K2_AddRelativeRotation` (`self.Turnpoint`) (`KismetMathLibrary.MakeRotator` 0.0 0.0 (`self.Rotation`)) false false)
  (if (and (not (`AudioComponent.IsPlaying` (`self.Speaker1`))) (`self.Playing`))
    (`self.Stop`)))

(event `Stop`
  (`|ExecutionSequence`
    (:`then_0`
      (`AudioComponent.FadeOut` (`self.Speaker1`) 0.2 0.0)
      (`AudioComponent.FadeOut` (`self.Speaker2`) 0.2 0.0))
    (:`then_1`
      (bind (_direction _newtrack_0) (`Timeline|StartRotation` :!via `Reverse` :!label _label)
        (:`Update`
          (set `self.Rotation` _newtrack_0))))
    (:`then_2`
      (bind (_direction_2 _rot) (`Timeline|NeedleRotation` :!via `Reverse` :!label _label_2)
        (:`Update`
          (`SceneComponent.K2_SetRelativeRotation` (`self.FBX_RecordPlayer_Hand`) (`KismetMathLibrary.MakeRotator` 0.0 0.0 (* _rot 10.0)) false false))))
    (:`then_3`
      (`KismetSystemLibrary.Delay` 6.0)
      (`KismetSystemLibrary.K2_ClearAndInvalidateTimerHandle` (stale `self.Box.OnComponentBeginOverlap` _returnvalue))
      (set `self.Playing` false)
      (set `self.CurrentRecord` null))))

(event `self.Box.OnComponentBeginOverlap`
  (params (OverlappedComponent :type "PrimitiveComponent Object Reference") (OtherActor :type "Actor Object Reference") (OtherComp :type "PrimitiveComponent Object Reference") (OtherBodyIndex :type Integer) (bFromSweep :type Boolean) (SweepResult :type "HitResult Structure (by ref)"))
  (bind _speaker2 (`self.Speaker2`))
  (bind _speaker1 (`self.Speaker1`))
  (bind _lp (`/Game/Blueprints/StationComponents/BP_Record.LP` (`self.CurrentRecord`)))
  (if (not (`self.Playing`))
    (bind _asbp_record (cast `/Game/Blueprints/StationComponents/BP_Record` OtherActor))
    (bind _output_get (set `self.CurrentRecord` _asbp_record))
    (`PrimitiveComponent.SetSimulatePhysics` (`/Game/Blueprints/StationComponents/Templates/BP_Interactable.Cube` _output_get) false)
    (set `/Game/Blueprints/StationComponents/Templates/BP_Grabbable.Pickupable` false _output_get)
    (`|ExecutionSequence`
      (:`then_0`
        (`self.K2_SetActorLocation` (`self.CurrentRecord`) (`SceneComponent.K2_GetComponentLocation` (`self.Turnpoint`)) false false)
        (`self.K2_AttachToComponent` (`self.CurrentRecord`) (`self.Turnpoint`) "None" "KeepWorld" "SnapToTarget" "KeepWorld" true)
        (`KismetSystemLibrary.Delay` 1.0)
        (goto _label_2))
      (:`then_1`
        (`KismetSystemLibrary.Delay` 2.0)
        (bind _returnvalue (`KismetSystemLibrary.K2_SetTimerDelegate` (delegate `RotateRecord`) 0.03 true))
        (goto _label))
      (:`then_2`
        (`KismetSystemLibrary.Delay` 10.0)
        (`AudioComponent.SetSound` _speaker1 _lp)
        (`AudioComponent.SetSound` _speaker2 _lp)
        (`AudioComponent.Play` _speaker1 0.0)
        (`AudioComponent.Play` _speaker2 0.0)
        (set `self.Playing` true)
        (set `/Game/Blueprints/StationComponents/Templates/BP_Grabbable.Pickupable` true (`self.CurrentRecord`))))))

(fn `UserConstructionScript`
  (`SceneComponent.K2_SetWorldLocation` (`self.Speaker1`) (`self.Speaker1Loc`) false false)
  (`SceneComponent.K2_SetWorldLocation` (`self.Speaker2`) (`self.Speaker2Loc`) false false))