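; BP_Sensor_ChipDrawer is a station component sensor that tracks two lock states for a chip drawer.
; UpdateLocks stores each lock's state and checks whether both are unlocked.
; Once both are unlocked, it disables its collision, spawns a BP_StandIn_ChipDrawer at its own transform and destroys itself, swapping the sensor for the stand-in.
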(event `UpdateLocks`
  (params (IsLock1 :type Boolean) (Unlocked :type Boolean))
  (if IsLock1
    (set `self.Lock1` Unlocked)
    (else
      (set `self.Lock2` Unlocked)))
  (if (and (`self.Lock1`) (`self.Lock2`))
    (if (not (`self.IsUnlocked`))
      (set `self.IsUnlocked` true)
      (`self.SetActorEnableCollision` false)
      (`|SpawnActorFromClass` "/Game/Blueprints/StationComponents/BP_StandIn_ChipDrawer.BP_StandIn_ChipDrawer_C" (`self.GetTransform`) "Undefined" "OverrideRootScale" null null)
      (`self.K2_DestroyActor`))
    (elif (`self.IsUnlocked`)
      (set `self.IsUnlocked` false))))

(fn `UserConstructionScript`)