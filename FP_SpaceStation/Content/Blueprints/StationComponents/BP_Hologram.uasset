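; BP_Hologram is a holographic model of a station whose outer body, solar arrays and rings can be shown or hidden by group.
; On BeginPlay, the RingRotation timeline spins the two rings in opposite yaw directions, the second offset by a quarter turn.
; Three events toggle each group's visibility, and the construction script calls them to start with body and solar arrays shown, rings hidden.
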(event `self.ReceiveBeginPlay`
  (bind (_direction _rot) (`Timeline|RingRotation`)
    (:`Update`
      (`SceneComponent.K2_SetRelativeRotation` (`self.Ring1`) (`KismetMathLibrary.MakeRotator` 0.0 0.0 (* _rot 360.0)) false false)
      (`SceneComponent.K2_SetRelativeRotation` (`self.Ring2`) (`KismetMathLibrary.MakeRotator` 0.0 0.0 (+ (* _rot -360.0) 90.0)) false false))))

(event `SetRingVisiblity`
  (params (Visible :type Boolean))
  (bind _returnvalue (not Visible))
  (`SceneComponent.SetHiddenInGame` (`self.Ring1`) _returnvalue false)
  (`SceneComponent.SetHiddenInGame` (`self.Ring2`) _returnvalue false))

(event `SetSolarPanelVisibility`
  (params (Visible :type Boolean))
  (bind _returnvalue (not Visible))
  (`SceneComponent.SetHiddenInGame` (`self.SolarArray1_1`) _returnvalue false)
  (`SceneComponent.SetHiddenInGame` (`self.SolarArray1_2`) _returnvalue false)
  (`SceneComponent.SetHiddenInGame` (`self.SolarArray2_1`) _returnvalue false)
  (`SceneComponent.SetHiddenInGame` (`self.SolarArray2_2`) _returnvalue false))

(event `SetOuterBodyVisibility`
  (params (Visible :type Boolean))
  (`SceneComponent.SetHiddenInGame` (`self.FBX_Holo_StationBody`) (not Visible) false))

(fn `UserConstructionScript`
  (`self.SetSolarPanelVisibility` true)
  (`self.SetRingVisiblity` false)
  (`self.SetOuterBodyVisibility` true))