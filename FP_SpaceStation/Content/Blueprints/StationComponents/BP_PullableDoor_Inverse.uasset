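; BP_PullableDoor_Inverse is a station component, by its name the inverse variant of a pullable door, and its only logic is a construction script.
; The script applies the configured mesh and physics-simulation setting to PullableObj, then sizes and positions BoxHandle from the grab scale and location variables.
; It finishes by calling SetMaterial on every slot with no material supplied, clearing any overrides.
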(fn `UserConstructionScript`
  (bind _pullableobj (`self.PullableObj`))
  (bind _box_handle (`self.Box_Handle`))
  (bind _pullableobj_2 (`self.PullableObj`))
  (`PrimitiveComponent.SetSimulatePhysics` _pullableobj (`self.SimulatePhysics`))
  (`StaticMeshComponent.SetStaticMesh` _pullableobj (`self.Mesh`))
  (`SceneComponent.SetRelativeScale3D` _box_handle (`self.GrabScale`))
  (`SceneComponent.K2_SetRelativeLocation` _box_handle (`self.GrabLoc`) false false)
  (for _index (range (`PrimitiveComponent.GetNumMaterials` _pullableobj_2))
    (`PrimitiveComponent.SetMaterial` _pullableobj_2 _index null)))