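; BP_HangingClothes is a station component for a pullable clothes hanger that can optionally carry a shirt.
; The construction script uses HasShirt to either apply the shirt material and swap the pullable object to the hanger part mesh, or hide the skeletal mesh.
; When a shirt is present, Tick moves the skeletal mesh to the pullable object's world location every frame.
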(event `self.ReceiveTick`
  (params (DeltaSeconds :type "Float (single-precision)"))
  (bind (_returnvalue_x _returnvalue_y _returnvalue_z) (`KismetMathLibrary.BreakVector` (`SceneComponent.K2_GetComponentLocation` (`self.PullableObj`))))
  (if (`self.HasShirt`)
    (`SceneComponent.K2_SetWorldLocation` (`self.SkeletalMesh`) (`KismetMathLibrary.MakeVector` _returnvalue_x _returnvalue_y _returnvalue_z) false false)))

(event `self.Update`)

(fn `UserConstructionScript`
  (bind _skeletalmesh (`self.SkeletalMesh`))
  (if (`self.HasShirt`)
    (`PrimitiveComponent.SetMaterial` _skeletalmesh 1 (`self.ShirtMat`))
    (`StaticMeshComponent.SetStaticMesh` (`self.PullableObj`) "/Game/Geometry/FBX_ClothesHanger_Part.FBX_ClothesHanger_Part")
    (else
      (`SceneComponent.SetVisibility` _skeletalmesh false false)
      (`SceneComponent.SetHiddenInGame` _skeletalmesh true false))))