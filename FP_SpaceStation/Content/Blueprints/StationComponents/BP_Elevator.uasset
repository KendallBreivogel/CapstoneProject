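; Space station elevator that can be called, dismissed and ridden between four floors.
; It registers as receiver on its child floor buttons and maps action numbers to call, dismiss, door and floor events.
; Timelines animate doors and car, slowing play rate for longer trips, while BP_SpaceStation changes floors with delayed unload.
; Overlap timers close doors after a pawn enters and dismiss the car after exit, closing elevator hatches.
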(event `self.ReceiveBeginPlay`
  (bind _asbp_button (cast `/Game/Blueprints/StationComponents/Templates/BP_Button` (`ChildActorComponent.ChildActor` (`self.Button_Command`))))
  (`KismetArrayLibrary.Array_Add` (`/Game/Blueprints/StationComponents/Templates/BP_Communicator.Reciever` _asbp_button) self)
  (bind _asbp_button_2 (cast `/Game/Blueprints/StationComponents/Templates/BP_Button` (`ChildActorComponent.ChildActor` (`self.Button_Lifestyle`))))
  (`KismetArrayLibrary.Array_Add` (`/Game/Blueprints/StationComponents/Templates/BP_Communicator.Reciever` _asbp_button_2) self)
  (bind _asbp_button_3 (cast `/Game/Blueprints/StationComponents/Templates/BP_Button` (`ChildActorComponent.ChildActor` (`self.Button_Hydroponics`))))
  (`KismetArrayLibrary.Array_Add` (`/Game/Blueprints/StationComponents/Templates/BP_Communicator.Reciever` _asbp_button_3) self)
  (bind _asbp_button_4 (cast `/Game/Blueprints/StationComponents/Templates/BP_Button` (`ChildActorComponent.ChildActor` (`self.Button_Outer`))))
  (`KismetArrayLibrary.Array_Add` (`/Game/Blueprints/StationComponents/Templates/BP_Communicator.Reciever` _asbp_button_4) self)
  (bind _outactors (`GameplayStatics.GetAllActorsOfClass` "/Game/Blueprints/BP_SpaceStation.BP_SpaceStation_C"))
  (bind _output_get (set `self.SpaceStation` (`|GetArrayItem` _outactors)))
  (`SceneComponent.K2_SetRelativeLocation` (`self.ElevatorMesh`) (`KismetMathLibrary.MakeVector` 0.0 0.0 (- (* (`/Game/Blueprints/BP_SpaceStation.CurrentFloor` _output_get) 630.0) 375.0)) false false))

(event `self.Action`
  (params (ActionNum :type Integer))
  (switch `int` ActionNum
    (:`0`
      (`self.Call`))
    (:`1`
      (`self.Dismiss`))
    (:`2`
      (`self.ToggleDoors`))
    (:`3`
      (`self.ChangeFloors` 0))
    (:`4`
      (`self.ChangeFloors` 1))
    (:`5`
      (`self.ChangeFloors` 2))
    (:`6`
      (`self.ChangeFloors` 3))))

(event `Call`
  (`KismetSystemLibrary.PrintString` "Call")
  (set `self.InUse` true)
  (bind (_direction _pos) (`Timeline|CallElevator` :!label _label)
    (:`Update`
      (`SceneComponent.K2_SetRelativeLocation` (`self.ElevatorMesh`) (`KismetMathLibrary.MakeVector` 0.0 0.0 (- (* (`/Game/Blueprints/BP_SpaceStation.CurrentFloor` (`self.SpaceStation`)) 630.0) (* _pos -375.0))) false false))
    (:`Finished`
      (if (`self.InUse`)
        (`self.OpenDoors`)
        (else
          (bind _outactors (`GameplayStatics.GetAllActorsOfClass` "/Game/Blueprints/StationComponents/BP_Module1_ElevatorHatch.BP_Module1_ElevatorHatch_C" :!label _label_2))
          (for _array_element _outactors
            (`/Game/Blueprints/StationComponents/BP_Module1_ElevatorHatch.Close` _array_element)))))))

(event `Dismiss`
  (`KismetSystemLibrary.PrintString` "Dismiss")
  (if (`self.InUse`)
    (set `self.InUse` false)
    (if (`self.DoorsOpen`)
      (`self.CloseDoors`))
    (`KismetSystemLibrary.Delay` 1.0)
    (goto _label :!via `Reverse`)
    (else
      (goto _label_2))))

(event `ToggleDoors`
  (if (`self.DoorsOpen`)
    (`self.CloseDoors`)
    (else
      (`self.OpenDoors`))))

(event `OpenDoors`
  (if (not (`self.DoorsOpen`))
    (set `self.DoorsOpen` true)
    (bind (_direction _pos) (`Timeline|Doors` :!label _label_3)
      (:`Update`
        (`SceneComponent.K2_SetRelativeRotation` (`self.DoorLeft`) (`KismetMathLibrary.MakeRotator` 0.0 0.0 (* _pos 50.0)) false false)
        (`SceneComponent.K2_SetRelativeRotation` (`self.DoorRight`) (`KismetMathLibrary.MakeRotator` 0.0 0.0 (* _pos -50.0)) false false)))))

(event `CloseDoors`
  (if (`self.DoorsOpen`)
    (set `self.DoorsOpen` false)
    (goto _label_3 :!via `Reverse`)))

(event `self.Box.OnComponentBeginOverlap`
  (params (OverlappedComponent :type "PrimitiveComponent Object Reference") (OtherActor :type "Actor Object Reference") (OtherComp :type "PrimitiveComponent Object Reference") (OtherBodyIndex :type Integer) (bFromSweep :type Boolean) (SweepResult :type "HitResult Structure (by ref)"))
  (cast `Pawn` OtherActor)
  (`KismetSystemLibrary.PrintString` "EnteredElevator")
  (bind _returnvalue (`KismetSystemLibrary.K2_SetTimerDelegate` (delegate `CloseDoors`) 2.0))
  (`KismetSystemLibrary.K2_ClearAndInvalidateTimerHandle` (stale `self.Box.OnComponentEndOverlap` _returnvalue)))

(event `self.Box.OnComponentEndOverlap`
  (params (OverlappedComponent :type "PrimitiveComponent Object Reference") (OtherActor :type "Actor Object Reference") (OtherComp :type "PrimitiveComponent Object Reference") (OtherBodyIndex :type Integer))
  (cast `Pawn` OtherActor)
  (`KismetSystemLibrary.PrintString` "ExitedElevator")
  (`KismetSystemLibrary.K2_ClearAndInvalidateTimerHandle` (stale `self.Box.OnComponentBeginOverlap` _returnvalue))
  (bind _returnvalue (`KismetSystemLibrary.K2_SetTimerDelegate` (delegate `Dismiss`) 2.0)))

(event `ChangeFloors`
  (params (NewFloor :type Integer))
  (bind _spacestation (`self.SpaceStation`))
  (bind _moveelevator (`self.MoveElevator`))
  (bind _currentfloor (`/Game/Blueprints/BP_SpaceStation.CurrentFloor` _spacestation))
  (set `self.TempFloor` _currentfloor)
  (switch `int` (`KismetMathLibrary.Abs_Int` (- NewFloor _currentfloor))
    (:`0`
      (`self.ToggleDoors`))
    (:`1`
      (`TimelineComponent.SetPlayRate` _moveelevator 0.5)
      (if (`self.DoorsOpen`) :!label _label_4
        (`self.CloseDoors`)
        (`KismetSystemLibrary.Delay` 1.0))
      (`/Game/Blueprints/BP_SpaceStation.ChangeFloors` _spacestation NewFloor 5.0)
      (bind (_direction _pos) (`Timeline|MoveElevator` :!via `PlayFromStart`)
        (:`Update`
          (`SceneComponent.K2_SetRelativeLocation` (`self.ElevatorMesh`) (`KismetMathLibrary.MakeVector` 0.0 0.0 (`KismetMathLibrary.Lerp` (* (`self.TempFloor`) 630.0) (* (`/Game/Blueprints/BP_SpaceStation.CurrentFloor` (`self.SpaceStation`)) 630.0) _pos)) false false))
        (:`Finished`
          (`self.OpenDoors`))))
    (:`2`
      (`TimelineComponent.SetPlayRate` _moveelevator 0.25)
      (goto _label_4))
    (:`3`
      (`TimelineComponent.SetPlayRate` _moveelevator 0.166)
      (goto _label_4))))

(fn `UserConstructionScript`)