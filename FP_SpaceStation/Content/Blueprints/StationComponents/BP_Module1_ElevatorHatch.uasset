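; Station elevator hatch whose two bulkhead leaves slide and rotate through a timeline, with sound on open and close.
; Action opens a closed hatch and calls the BP_Elevator once the animation finishes open.
; On an open hatch, it forwards to the elevator if that is in use, otherwise closes.
; Opening snaps all other hatches open instantly, while closing triggers their animated close.
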(event `self.ReceiveBeginPlay`
  (bind _outactors (`GameplayStatics.GetAllActorsOfClass` "/Game/Blueprints/StationComponents/BP_Elevator.BP_Elevator_C"))
  (set `self.Elevator` (`|GetArrayItem` _outactors))
  (if (`self.IsOpen`)
    (`self.OpenInstant`)
    (else
      (`self.CloseInstant`))))

(event `OpenInstant`
  (`TimelineComponent.SetNewTime` (`self.OpenBulkheads`) 2.0)
  (set `self.IsOpen` true))

(event `CloseInstant`
  (`TimelineComponent.SetNewTime` (`self.OpenBulkheads`) 0.0)
  (set `self.IsOpen` false))

(event `self.Action`
  (params (ActionNum :type Integer))
  (bind _returnvalue (`self.K2_GetActorLocation`))
  (bind _left (`self.Left`))
  (bind _right (`self.Right`))
  (bind _elevator (`self.Elevator`))
  (if (`self.IsOpen`)
    (if (`/Game/Blueprints/StationComponents/BP_Elevator.InUse` _elevator)
      (`self.Action` _elevator 1)
      (else
        (`KismetSystemLibrary.Delay` 0.5 :!label _label)
        (set `self.IsOpen` false)
        (`self.CloseAllHatches`)
        (`KismetSystemLibrary.PrintString` "CloseHatch")
        (`GameplayStatics.PlaySoundAtLocation` "/Game/Audio/WAV_Elevator_HatchClose.WAV_Elevator_HatchClose" _returnvalue (struct) 0.5 1.0 0.0 "/Game/Audio/BasicAttenuation.BasicAttenuation" null null)
        (bind (_direction _height _rot) (`Timeline|OpenBulkheads` :!via `Reverse` :!label _label_2)
          (:`Update`
            (`SceneComponent.K2_SetRelativeLocation` _left (`KismetMathLibrary.MakeVector` 0.0 (* _height -80.0)) false false)
            (`SceneComponent.K2_SetRelativeLocation` _right (`KismetMathLibrary.MakeVector` 0.0 (* _height 80.0)) false false)
            (bind _returnvalue_2 (* _rot 90.0))
            (`SceneComponent.K2_SetRelativeRotation` _left (`KismetMathLibrary.MakeRotator` 0.0 0.0 _returnvalue_2) false false)
            (`SceneComponent.K2_SetRelativeRotation` _right (`KismetMathLibrary.MakeRotator` 0.0 0.0 _returnvalue_2) false false))
          (:`Finished`
            (if (`self.IsOpen`)
              (`self.Action` (`self.Elevator`) 0))))))
    (else
      (`KismetSystemLibrary.Delay` 0.5 :!label _label_3)
      (set `self.IsOpen` true)
      (`self.OpenAllHatches`)
      (`KismetSystemLibrary.PrintString` "OpenHatch")
      (`GameplayStatics.PlaySoundAtLocation` "/Game/Audio/WAV_Elevator_Hatch.WAV_Elevator_Hatch" _returnvalue (struct) 0.5 1.0 0.0 "/Game/Audio/BasicAttenuation.BasicAttenuation" null null)
      (goto _label_2))))

(event `Open`
  (goto _label_3))

(event `Close`
  (goto _label))

(fn `CloseAllHatches`
  (bind _outactors (`GameplayStatics.GetAllActorsOfClass` "BP_Module1_ElevatorHatch_C"))
  (for _array_element _outactors
    (if (`/Game/Blueprints/StationComponents/BP_Module1_ElevatorHatch.IsOpen` _array_element)
      (`self.Close` _array_element))))

(fn `OpenAllHatches`
  (bind _outactors (`GameplayStatics.GetAllActorsOfClass` "BP_Module1_ElevatorHatch_C"))
  (for _array_element _outactors
    (if (not (`/Game/Blueprints/StationComponents/BP_Module1_ElevatorHatch.IsOpen` _array_element))
      (`self.OpenInstant` _array_element))))

(fn `UserConstructionScript`
  (bind _staticmesh3 (`self.StaticMesh3`))
  (bind _staticmesh2 (`self.StaticMesh2`))
  (if (not (`self.HasTop`))
    (`SceneComponent.SetHiddenInGame` _staticmesh3 false false)
    (`SceneComponent.SetHiddenInGame` _staticmesh2 false false)
    (`SceneComponent.SetVisibility` _staticmesh3 false false)
    (`SceneComponent.SetVisibility` _staticmesh2 false false)))