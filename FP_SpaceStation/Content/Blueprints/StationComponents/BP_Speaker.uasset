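; BP_Speaker is a station component that plays a requested sound through its Audio component.
; PlaySound swaps in the sound, fades it in briefly, marks the speaker in use and flags whether the sound is the alarm.
; StopSound acts only while the speaker is in use, fading the audio out and clearing both flags.
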(event `PlaySound`
  (params (Sound :type "SoundWave Object Reference"))
  (bind _audio (`self.Audio`))
  (`AudioComponent.SetSound` _audio Sound)
  (`AudioComponent.FadeIn` _audio 0.25 1.0 0.0)
  (set `self.InUse` true)
  (if (== Sound "/Game/Audio/WAV_Alarm.WAV_Alarm")
    (set `self.Alarm` true)
    (else
      (set `self.Alarm` false))))

(event `StopSound`
  (if (`self.InUse`)
    (`AudioComponent.FadeOut` (`self.Audio`) 0.5 0.0)
    (set `self.InUse` false)
    (set `self.Alarm` false)))

(fn `UserConstructionScript`)