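; Space station manager that spins the outer rings and controls the current module's status and floor streaming.
; LocateCurrentModule finds the current floor's mesh, lights, speaker and bulkheads by actor tag.
; StatusChange drives a dynamic emissive material, light color and flashing, and the Danger alarm, by timeline or instantly, with bulkheads updating only on instant changes.
; ChangeFloors optionally streams levels, unloading the previous after a delay, then reapplies status.
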(event `self.ReceiveBeginPlay`
  (`|ExecutionSequence`
    (:`then_0`
      (`KismetSystemLibrary.Delay` 0.5)
      (`self.LocateCurrentModule`)
      (`self.StatusChange` "NewEnumerator3"))
    (:`then_1`
      (bind (_direction _rot) (`Timeline|RingRotation` :!via `PlayFromStart`)
        (:`Update`
          (`SceneComponent.K2_SetRelativeRotation` (`self.FBX_SS_OuterRing1`) (`KismetMathLibrary.MakeRotator` 0.0 0.0 (* _rot 360.0)) false false)
          (`SceneComponent.K2_SetRelativeRotation` (`self.FBX_SS_OuterRing2`) (`KismetMathLibrary.MakeRotator` 0.0 0.0 (+ (* _rot -360.0) 90.0)) false false))))))

(event `StatusChange`
  (params (NewStatus :type "/Game/Blueprints/Status Enum" :default "NewEnumerator0") (Instant :type Boolean))
  (bind _dynamicstatusmat (`self.DynamicStatusMat`))
  (bind _dynamicstatusmat_2 (`self.DynamicStatusMat`))
  (bind _currentstatuscolor (`self.CurrentStatusColor`))
  (bind _currentmodulebulkheads (`self.CurrentModuleBulkheads`))
  (bind _currentmodulelight (`self.CurrentModuleLight`))
  (set `self.StationStatus` NewStatus)
  (set `self.TempStatusColor` (`self.CurrentStatusColor`))
  (switch `/Game/Blueprints/Status` (`self.StationStatus`)
    (:`NewEnumerator0`
      (set `self.IsLockedDown` false)
      (set `self.CurrentStatusColor` (struct :`R` 0.262745 :`G` 0.462745 :`B` 1.0 :`A` 1.0))
      (`MaterialInstanceDynamic.SetScalarParameterValue` _dynamicstatusmat "Flashing" 0.0 :!label _label)
      (`|ExecutionSequence`
        (:`then_0`
          (if Instant :!label _label_2
            (`MaterialInstanceDynamic.SetVectorParameterValue` _dynamicstatusmat_2 "EmissiveColor" _currentstatuscolor)
            (for _array_element _currentmodulelight
              (`LightComponent.SetLightColor` (`PointLight.PointLightComponent` _array_element) (`self.Desaturate` _currentstatuscolor 0.9) true)
              (if (`self.IsLockedDown`)
                (`/Game/Blueprints/StationComponents/BP_Module1_Bulkheads.CloseInstant` _currentmodulebulkheads)
                (else
                  (`/Game/Blueprints/StationComponents/BP_Module1_Bulkheads.OpenInstant` _currentmodulebulkheads))))
            (else
              (bind (_direction _trans) (`Timeline|ColorTransition` :!via `PlayFromStart`)
                (:`Update`
                  (bind _returnvalue (`KismetMathLibrary.LinearColorLerp` (`self.TempStatusColor`) _currentstatuscolor _trans))
                  (`MaterialInstanceDynamic.SetVectorParameterValue` _dynamicstatusmat_2 "EmissiveColor" _returnvalue)
                  (for _array_element_2 _currentmodulelight
                    (`LightComponent.SetLightColor` (`PointLight.PointLightComponent` _array_element_2) (`self.Desaturate` _returnvalue 0.9) true)))))))
        (:`then_1`
          (bind (_direction_2 _plintensity) (`Timeline|FlashingLight` :!via `Stop` :!label _label_3)
            (:`Update`
              (for _array_element_3 (`self.CurrentModuleLight`)
                (`LightComponent.SetIntensity` (`PointLight.PointLightComponent` _array_element_3) (* _plintensity 2.0))))))
        (:`then_2`
          (`self.StopAlarm`))))
    (:`NewEnumerator1`
      (set `self.IsLockedDown` false)
      (set `self.CurrentStatusColor` (struct :`R` 1.0 :`A` 1.0))
      (`MaterialInstanceDynamic.SetScalarParameterValue` _dynamicstatusmat "Flashing" 1.0)
      (`|ExecutionSequence`
        (:`then_0`
          (goto _label_2))
        (:`then_1`
          (goto _label_3 :!via `PlayFromStart`))
        (:`then_2`
          (`self.StartAlarm`))))
    (:`NewEnumerator2`
      (set `self.IsLockedDown` false)
      (set `self.CurrentStatusColor` (struct :`R` 1.0 :`G` 0.482353 :`B` 0.160784 :`A` 1.0))
      (goto _label))
    (:`NewEnumerator3`
      (set `self.IsLockedDown` true)
      (set `self.CurrentStatusColor` (struct :`R` 1.0 :`G` 0.450786 :`A` 1.0))
      (goto _label))))

(event `StartAlarm`
  (bind _audio (`/Game/Blueprints/StationComponents/BP_Speaker.Audio` (`self.CurrentModuleSpeaker`)))
  (`AudioComponent.SetSound` _audio "/Game/Audio/WAV_Alarm.WAV_Alarm")
  (`AudioComponent.FadeIn` _audio 0.25 1.0 0.0))

(event `StopAlarm`
  (`AudioComponent.FadeOut` (`/Game/Blueprints/StationComponents/BP_Speaker.Audio` (`self.CurrentModuleSpeaker`)) 0.5 0.0))

(event `ChangeFloors`
  (params (NewFloor :type Integer) (UnloadDelay :type "Float (double-precision)"))
  (set `self.PreviousFloor` (`self.CurrentFloor`))
  (if (`self.DoUnloadLevels`)
    (`|ExecutionSequence`
      (:`then_0`
        (switch `int` NewFloor
          (:`0`
            (`GameplayStatics.LoadStreamLevel` "HydroponicsModule" true true)
            (set `self.CurrentFloor` 0))
          (:`1`
            (`GameplayStatics.LoadStreamLevel` "LifestyleModule" true true)
            (set `self.CurrentFloor` 1))
          (:`2`
            (`GameplayStatics.LoadStreamLevel` "CommandModule" true true)
            (set `self.CurrentFloor` 2))
          (:`3`
            (`GameplayStatics.LoadStreamLevel` "Outer" true true)
            (set `self.CurrentFloor` 3)))
        (`self.LocateCurrentModule` :!label _label_4)
        (`self.StatusChange` (`self.StationStatus`) true))
      (:`then_1`
        (`KismetSystemLibrary.Delay` UnloadDelay)
        (switch `int` (`self.PreviousFloor`)
          (:`0`
            (`GameplayStatics.UnloadStreamLevel` "HydroponicsModule"))
          (:`1`
            (`GameplayStatics.UnloadStreamLevel` "LifestyleModule"))
          (:`2`
            (`GameplayStatics.UnloadStreamLevel` "CommandModule"))
          (:`3`
            (`GameplayStatics.UnloadStreamLevel` "Outer")))))
    (else
      (set `self.CurrentFloor` NewFloor)
      (goto _label_4))))

(fn `LocateCurrentModule`
  (returns (Success :type Boolean))
  (bind _currenttag (`self.CurrentTag`))
  (bind _returnvalue (`KismetStringLibrary.Conv_NameToString` _currenttag))
  (`KismetArrayLibrary.Array_Clear` (`self.CurrentModuleLight`))
  (switch `int` (`self.CurrentFloor`)
    (:`0`
      (set `self.CurrentTag` "HydroponicsModule"))
    (:`1`
      (set `self.CurrentTag` "LifestyleModule"))
    (:`2`
      (set `self.CurrentTag` "CommandModule")))
  (`|ExecutionSequence`
    (:`then_0`
      (bind _outactors (`GameplayStatics.GetAllActorsWithTag` _currenttag))
      (bind _asstatic_mesh_actor (cast `StaticMeshActor` (`|GetArrayItem` _outactors)))
      (bind _output_get (set `self.CurrentModule` _asstatic_mesh_actor))
      (`PrimitiveComponent.SetMaterialByName` (`StaticMeshActor.StaticMeshComponent` _output_get) "EmissiveMaster" (`self.DynamicStatusMat`))
      (`KismetSystemLibrary.PrintString` (`KismetSystemLibrary.GetDisplayName` _asstatic_mesh_actor)))
    (:`then_1`
      (bind _outactors_2 (`GameplayStatics.GetAllActorsWithTag` (`KismetStringLibrary.Conv_StringToName` (`KismetStringLibrary.Concat_StrStr` _returnvalue "Coll"))))
      (bind _asstatic_mesh_actor_2 (cast `StaticMeshActor` (`|GetArrayItem` _outactors_2)))
      (set `self.CurrentModuleColl` _asstatic_mesh_actor_2))
    (:`then_2`
      (bind _outactors_3 (`GameplayStatics.GetAllActorsWithTag` (`KismetStringLibrary.Conv_StringToName` (`KismetStringLibrary.Concat_StrStr` _returnvalue "Light"))))
      (for _array_element _outactors_3
        (bind _aspoint_light (cast `PointLight` _array_element))
        (`KismetArrayLibrary.Array_Add` (`self.CurrentModuleLight`) _aspoint_light)))
    (:`then_3`
      (bind _outactors_4 (`GameplayStatics.GetAllActorsOfClass` "/Game/Blueprints/StationComponents/BP_Speaker.BP_Speaker_C"))
      (for _array_element_2 _outactors_4
        (if (`self.ActorHasTag` _array_element_2 (`KismetStringLibrary.Conv_StringToName` (`KismetStringLibrary.Concat_StrStr` _returnvalue "Speaker")))
          (set `self.CurrentModuleSpeaker` _array_element_2))))
    (:`then_4`
      (bind _outactors_5 (`GameplayStatics.GetAllActorsOfClass` "/Game/Blueprints/StationComponents/BP_Module1_Bulkheads.BP_Module1_Bulkheads_C"))
      (for _array_element_3 _outactors_5
        (if (`self.ActorHasTag` _array_element_3 (`KismetStringLibrary.Conv_StringToName` (`KismetStringLibrary.Concat_StrStr` _returnvalue "Bulkheads")))
          (set `self.CurrentModuleBulkheads` _array_element_3))))
    (:`then_5`
      (return (and (`KismetSystemLibrary.IsValid` (`self.CurrentModule`)) (`KismetSystemLibrary.IsValid` (`self.CurrentModuleColl`)) (> (`KismetArrayLibrary.Array_Length` (`self.CurrentModuleLight`)) 0) (`KismetSystemLibrary.IsValid` (`self.CurrentModuleSpeaker`)) (`KismetSystemLibrary.IsValid` (`self.CurrentModuleBulkheads`)))))))

(fn `UserConstructionScript`
  (bind _returnvalue (`KismetMaterialLibrary.CreateDynamicMaterialInstance` "/Game/Materials/M_Emissive_Master.M_Emissive_Master"))
  (set `self.DynamicStatusMat` _returnvalue))